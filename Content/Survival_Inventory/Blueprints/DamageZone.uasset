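; DamageZone is a trigger area that deals periodic damage to players standing inside it.
; Overlap begin and end events add and remove actors from an Actors array on the server authority only.
; A looping one-second timer casts each tracked actor to ThirdPersonCharacter and calls DamageTaken on its PlayerInventoryComponent, removing entries whose component is invalid.
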(event OnComponentBeginOverlap(DamageZone)
  (params (OverlappedComponent :type Primitive%20Component%20Object%20Reference) (OtherActor :type Actor%20Object%20Reference) (OtherComp :type Primitive%20Component%20Object%20Reference) (OtherBodyIndex :type Integer) (bFromSweep :type Boolean) (SweepResult :type Hit%20Result%20Structure%20%28by%20ref%29))
  ;[1 1 1] Add and remove actors to array
  (Networking|SwitchHasAuthority
    (:Authority
      (Utilities|Array|Add (Variables|Default|GetActors) OtherActor))))

(event OnComponentEndOverlap(DamageZone)
  (params (OverlappedComponent :type Primitive%20Component%20Object%20Reference) (OtherActor :type Actor%20Object%20Reference) (OtherComp :type Primitive%20Component%20Object%20Reference) (OtherBodyIndex :type Integer))
  ;[1 1 1] Add and remove actors to array
  (Networking|SwitchHasAuthority
    (:Authority
      (Utilities|Array|RemoveItem (Variables|Default|GetActors) OtherActor))))

(event Custom|Damage
  ;[1 1 1] Apply damage to players
  (for _array_element (Variables|Default|GetActors)
    (bind _asthird_person_character (Utilities|Casting|CastToThirdPersonCharacter _array_element))
    (Utilities|IsValid (Variables|/Game/Survival_Inventory/Blueprints/ThirdPersonCharacter.ThirdPersonCharacter_C|GetPlayerInventoryComponent _asthird_person_character)
      (:Is%20Valid
        (Default|DamageTaken (Variables|/Game/Survival_Inventory/Blueprints/ThirdPersonCharacter.ThirdPersonCharacter_C|GetPlayerInventoryComponent _asthird_person_character) 10))
      (:Is%20Not%20Valid
        (Utilities|Array|RemoveItem (Variables|Default|GetActors) _array_element)))))

(event EventBeginPlay
  ;[1 1 1] Apply damage to players
  (Utilities|Time|SetTimerbyEvent (delegate Custom|Damage) 1.0 true))

(fn ConstructionScript)