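; World pickup actor for an inventory item, which a player collects by interacting with it.
; The construction script and an all-client spawn event set the world mesh from the item's looked-up details.
; Interaction, called on the server, passes the actor to the player component's server pickup call, and a separate event destroys it on all clients.
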(event Custom|Destroy%20Item
  ;[1 1 1] All clients destroy item
  (Actor|DestroyActor))

(event Custom|On%20Spawned
  ;[1 1 1] All clients on spawned set static mesh
  (Components|StaticMesh|SetStaticMesh (Variables|Default|GetItem%20World%20Mesh) (.WorldMesh (Utilities|Struct|BreakS_ItemDetails (.Item%20Details%20Out (CallFunction|ItemDetails (Variables|Default|GetItem)))))))

(event EventInteract
  (params (Player%20Component :type Player%20Inventory%20Component%20Object%20Reference))
  ;[1 1 1] Server calls interact
  (Default|ServerPickupItem Player%20Component self))

(fn ConstructionScript
  (bind _item (Variables|Default|GetItem))
  (bind (_return_value _item_details_out) (CallFunction|ItemDetails _item))
  (if _return_value
    (Components|StaticMesh|SetStaticMesh (Variables|Default|GetItem%20World%20Mesh) (.WorldMesh (Utilities|Struct|BreakS_ItemDetails _item_details_out)))))